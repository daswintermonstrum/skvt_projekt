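; EMP sparks effect Blueprint that pairs a spark particle system with an EMP explosion component.
; EmpPressed activates the sparks, then deactivates them after a short random delay, ignoring its PressedOn input.
; The construction script calls EmpPressed and applies separate visibility flags to the sparks and explosion.
; EmpToggleOn sets both flags from one input and shows or hides both components together.
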(event Custom|EmpPressed
  (params (PressedOn :type Boolean))
  (Components|Activation|Activate (Variables|Emitter|GetParticleSystemComponent) false)
  (Utilities|FlowControl|Delay (Math|Random|RandomFloatinRange 0.3 1.0))
  (Components|Activation|Deactivate (Variables|Emitter|GetParticleSystemComponent)))

(fn ConstructionScript
  (CallFunction|EmpPressed false)
  (Rendering|SetVisibility (Variables|Emitter|GetParticleSystemComponent) (Variables|Default|GetEmpOnOff) false)
  (Rendering|SetVisibility (Variables|Default|GetP_Explosion_EMP) (Variables|Default|GetExplosionOnOff) false))

(fn EmpToggleon
  (params (Is%20On :type Boolean))
  (bind _output_get (Variables|Default|SetEmpOnOff Is%20On))
  (bind _output_get_2 (Variables|Default|SetExplosionOnOff _output_get))
  (Rendering|SetVisibility (Variables|Emitter|GetParticleSystemComponent) _output_get_2 false)
  (Rendering|SetVisibility (Variables|Default|GetP_Explosion_EMP) _output_get_2 false))