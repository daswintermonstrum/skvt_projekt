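; BP_WallSconceEMP is a wall sconce light that can be switched on and off electrically or broken.
; The construction script sets a fixed intensity and applies the color, cone angles and on/off visibility variables.
; ToggleonElectric sets visibility through an internal function.
; LightBreaking reduces the Brightness variable without applying it to the light, then switches the light off after a short random delay.
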(event Custom|Light%20Breaking
  (params (Started%20Breaking :type Boolean))
  (Variables|Light|SetBrightness (* (Variables|Light|GetBrightness) 0.2))
  (Utilities|FlowControl|Delay (Math|Random|RandomFloatinRange 0.3 1.0))
  (CallFunction|ToggleonElectricInternal false)
  (Variables|Light|SetOnOff false))

(event EventToggleonElectric
  (params (IsOn :type Boolean))
  (CallFunction|ToggleonElectricInternal IsOn))

(fn ConstructionScript
  (bind _sconcelight (Variables|Default|GetSconceLight))
  (Rendering|Components|Light|SetIntensity _sconcelight 1e+03)
  (Rendering|Components|Light|SetLightColor _sconcelight (Variables|Light|GetColor) true)
  (Rendering|Lighting|SetInnerConeAngle _sconcelight (Variables|Light|GetInner%20Cone%20Angle))
  (Rendering|Lighting|SetOuterConeAngle _sconcelight (Variables|Light|GetOuter%20Cone%20Angle))
  (Rendering|SetVisibility _sconcelight (Variables|Light|GetOnOff) false))

(fn ToggleonElectricInternal
  (params (IsOn :type Boolean))
  (bind _output_get (Variables|Light|SetOnOff IsOn))
  (Rendering|SetVisibility (Variables|Default|GetSconceLight) _output_get false))