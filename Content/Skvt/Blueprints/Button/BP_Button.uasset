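; BP_Button is an interactable button that sets off an EMP, breaking lights and activating emitters.
; On Interact, if TurnInteractOff is true, it calls LightBreaking on the LightsEMP entries and sets EmpPressed and EmpToggleOn on the Emmiter entries in a nested loop.
; After a two-second delay it adds a particle system and clears TurnInteractOff, which blocks later interactions.
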(event EventInteract
  (bind _lightsemp (Variables|Default|GetLightsEMP))
  (if (Variables|Default|GetTurnInteractOff)
    (for _array_element _lightsemp
      (Default|LightBreaking _lightsemp true)
      (for _array_element_2 (Variables|Default|GetEmmiter)
        (Default|EmpPressed _array_element_2 true)
        (Default|EmpToggleon _array_element_2 true)
        (Utilities|FlowControl|Delay 2.0)
        (AddComponent|AddParticleSystemComponent false)
        (Variables|Default|SetTurnInteractOff false))
      (Default|EmpPressed _array_element_2 true)
      (Default|EmpToggleon _array_element_2 true)
      (Utilities|FlowControl|Delay 2.0)
      (AddComponent|AddParticleSystemComponent false)
      (Variables|Default|SetTurnInteractOff false))
    (Default|LightBreaking _lightsemp true)
    (for _array_element_3 (Variables|Default|GetEmmiter)
      (Default|EmpPressed _array_element_3 true)
      (Default|EmpToggleon _array_element_3 true)
      (Utilities|FlowControl|Delay 2.0)
      (AddComponent|AddParticleSystemComponent false)
      (Variables|Default|SetTurnInteractOff false))
    (Default|EmpPressed _array_element_3 true)
    (Default|EmpToggleon _array_element_3 true)
    (Utilities|FlowControl|Delay 2.0)
    (AddComponent|AddParticleSystemComponent false)
    (Variables|Default|SetTurnInteractOff false)))

(fn ConstructionScript)