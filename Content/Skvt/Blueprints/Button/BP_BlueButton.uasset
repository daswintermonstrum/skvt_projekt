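; BP_BlueButton is an overlap-driven button that switches linked electric devices.
; An actor entering its overlap sends each entry in ElectricDevices a ToggleOnElectricMessage of false, and leaving sends true.
; Both events also set TurnInteractOff to true for each device processed, never resetting it.
; A disconnected chain that would trigger EMP emitters, delay and add a particle system never runs.
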(event Collision|EventActorBeginOverlap
  (params (OtherActor :type Actor%20Object%20Reference))
  (for _array_element (Variables|Default|GetElectricDevices)
    (Class|BPIElectric|ToggleonElectric(Message) _array_element false)
    (Variables|Default|SetTurnInteractOff true)))

(event Collision|EventActorEndOverlap
  (params (OtherActor :type Actor%20Object%20Reference))
  (for _array_element (Variables|Default|GetElectricDevices)
    (Class|BPIElectric|ToggleonElectric(Message) _array_element true)
    (Variables|Default|SetTurnInteractOff true)))

(fn ConstructionScript)