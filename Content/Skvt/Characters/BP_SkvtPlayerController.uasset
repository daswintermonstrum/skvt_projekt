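; Player controller that sets up Enhanced Input, lets the player swap between characters and toggles a pausing main menu.
; BeginPlay adds the default, swap, camera and crouch mapping contexts at equal priority.
; The swap action finds the possessed BP_SkvtBaseChar among all actors of that class and possesses the next, wrapping to the first.
; The menu action creates or removes WBP_MainMenu, switching cursor, input mode and pause state.
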(event Input|EnhancedActionEvents|EnhancedInputActionIA_Swap
  (params (ActionValue :type Boolean) (ElapsedSeconds :type Float%20%28double-precision%29) (TriggeredSeconds :type Float%20%28double-precision%29) (InputAction :type Input%20Action%20Object%20Reference :default "/Game/Skvt/Characters/Input/Actions/IA_Swap.IA_Swap"))
  (:Triggered
    (bind _outactors (Actor|GetAllActorsOfClass "/Game/Skvt/Characters/BP_SkvtBaseChar.BP_SkvtBaseChar_C"))
    (bind _asbp_skvt_base_char (Utilities|Casting|CastToBP_SkvtBaseChar (Pawn|GetControlledPawn)))
    (if (>= (Utilities|Array|FindItem _outactors _asbp_skvt_base_char) 0)
      (if (== (Utilities|Array|Length _outactors) (+ (Utilities|Array|FindItem _outactors _asbp_skvt_base_char) 1))
        (Pawn|Possess (Utilities|Array|Get(acopy) _outactors))
        (else
          (Pawn|Possess (Utilities|Array|Get(acopy) _outactors (+ (Utilities|Array|FindItem _outactors _asbp_skvt_base_char) 1))))))))

(event Input|EnhancedActionEvents|EnhancedInputActionIA_ToggleOpenMenu
  (params (ActionValue :type Boolean) (ElapsedSeconds :type Float%20%28double-precision%29) (TriggeredSeconds :type Float%20%28double-precision%29) (InputAction :type Input%20Action%20Object%20Reference :default "/Game/Skvt/Characters/Input/Actions/IA_ToggleOpenMenu.IA_ToggleOpenMenu"))
  (:Triggered
    (if (CallFunction|IsMenuOpen)
      (CallFunction|CloseMenu)
      (else
        (CallFunction|OpenMenu)))))

(event EventBeginPlay
  (bind _self self)
  (bind _returnvalue (PlayerController|LocalPlayerSubsystems|GetEnhancedInputLocalPlayerSubsystem _self))
  (Utilities|IsValid _returnvalue
    (:Is%20Valid
      (Input|AddMappingContext _returnvalue "/Game/ThirdPerson/Input/IMC_Default.IMC_Default" 0 "(bIgnoreAllPressedKeysUntilRelease=True,bForceImmediately=False)")
      (Input|AddMappingContext _returnvalue "/Game/Skvt/Characters/Input/IMC_SwapPawn.IMC_SwapPawn" 0 "(bIgnoreAllPressedKeysUntilRelease=True,bForceImmediately=False)")
      (Input|AddMappingContext _returnvalue "/Game/Skvt/Characters/Input/IMC_Camera.IMC_Camera" 0 "(bIgnoreAllPressedKeysUntilRelease=True,bForceImmediately=False)")
      (Input|AddMappingContext _returnvalue "/Game/Skvt/Characters/Input/IMC_Crouch.IMC_Crouch" 0 "(bIgnoreAllPressedKeysUntilRelease=True,bForceImmediately=False)"))))

(fn ConstructionScript)

(fn IsMenuOpen
  (Utilities|IsValid (Variables|Default|GetMainMenuRef)
    (:Is%20Valid
      (return true))
    (:Is%20Not%20Valid
      (return false))))

(fn OpenMenu
  (bind _returnvalue (UserInterface|CreateWidget "/Game/Skvt/UI/Widgets/Menu/WBP_MainMenu.WBP_MainMenu_C" self))
  (bind _output_get (Variables|Default|SetMainMenuRef _returnvalue))
  (UserInterface|Viewport|AddtoViewport _output_get 0)
  (Variables|Default|SetbShowMouseCursor true)
  (Input|SetInputModeGameandUI self 0 "DoNotLock" true false)
  (Game|SetGamePaused true))

(fn CloseMenu
  (Utilities|IsValid (Variables|Default|GetMainMenuRef)
    (:Is%20Valid
      (Widget|RemovefromParent (Variables|Default|GetMainMenuRef))
      (Variables|Default|SetMainMenuRef 0)
      (Variables|Default|SetbShowMouseCursor false)
      (Input|SetInputModeGameOnly self false)
      (Game|SetGamePaused false))))